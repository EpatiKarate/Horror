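; Objective trigger box that sets the player's objective to "Deal with the Razorz!" when BP_Trauma overlaps it.
; On overlap it updates the character's objective, then loads the HostileRealitySaveGame slot, or creates a new save object if none exists.
; It writes the same objective into the save, saves it to the slot and prints the result.
; The trigger has no one-shot guard in its graph.
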(event `self.ReceiveActorBeginOverlap`
  (params (OtherActor :type "Actor Object Reference"))
  (bind _savesubclass (`self.SaveSubClass`))
  (bind _asbp_trauma (cast `/Game/CharactersAndWeapons/Blueprint/BP_Trauma` OtherActor))
  (set `/Game/CharactersAndWeapons/Blueprint/BP_Trauma.PlayerObjective` "Deal with the Razorz!" _asbp_trauma)
  (bind _returnvalue (`GameplayStatics.DoesSaveGameExist` "HostileRealitySaveGame"))
  (if _returnvalue
    (bind _returnvalue_2 (`GameplayStatics.LoadGameFromSlot` "HostileRealitySaveGame"))
    (bind _output_get (set `self.SaveSubClass` _returnvalue_2))
    (bind _ashostile_reality_save_game (cast `/Game/CharactersAndWeapons/Blueprint/HostileRealitySaveGame` _output_get))
    (set `/Game/CharactersAndWeapons/Blueprint/HostileRealitySaveGame.PlayerObj` "Deal with the Razorz!" _ashostile_reality_save_game)
    (bind _returnvalue_3 (`GameplayStatics.SaveGameToSlot` _savesubclass "HostileRealitySaveGame"))
    (`KismetSystemLibrary.PrintString` (`KismetStringLibrary.Conv_BoolToString` _returnvalue_3))
    (else
      (bind _returnvalue_4 (`GameplayStatics.CreateSaveGameObject` "/Game/CharactersAndWeapons/Blueprint/HostileRealitySaveGame.HostileRealitySaveGame_C"))
      (bind _output_get_2 (set `self.SaveSubClass` _returnvalue_4))
      (bind _ashostile_reality_save_game_2 (cast `/Game/CharactersAndWeapons/Blueprint/HostileRealitySaveGame` _output_get_2))
      (set `/Game/CharactersAndWeapons/Blueprint/HostileRealitySaveGame.PlayerObj` "Deal with the Razorz!" _ashostile_reality_save_game_2)
      (bind _returnvalue_5 (`GameplayStatics.SaveGameToSlot` _savesubclass "HostileRealitySaveGame"))
      (`KismetSystemLibrary.PrintString` (`KismetStringLibrary.Conv_BoolToString` _returnvalue_5)))))

(fn `UserConstructionScript`)