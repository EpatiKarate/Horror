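; Master projectile Blueprint that applies location-based damage when it overlaps a damageable NPC.
; The hit location comes from a line trace along the player camera's view at overlap time, not from the projectile itself.
; The headshot component and hit bone names scale Damage through an if-chain, with a debug print per zone.
; Lethal headshot and chest hits play death animations on the NPC mesh.
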(event `self.ReceiveActorBeginOverlap`
  (params (OtherActor :type "Actor Object Reference"))
  (bind _returnvalue (`GameplayStatics.GetPlayerCameraManager` 0))
  (bind _returnvalue_2 (`self.K2_GetActorLocation` _returnvalue))
  (bind _asnpc (cast `/Game/CharactersAndWeapons/Blueprint/AI/NPC` OtherActor))
  (if (`Actor.bCanBeDamaged` OtherActor)
    (bind _outhit (`KismetSystemLibrary.LineTraceSingle` :`Start` _returnvalue_2 :`End` (+ _returnvalue_2 (* (`KismetMathLibrary.GetForwardVector` (`self.K2_GetActorRotation` _returnvalue)) 1000000.0)) :`TraceChannel` "TraceTypeQuery1" :`DrawDebugType` "ForOneFrame"))
    (bind (_bblockinghit _binitialoverlap _time _distance _location _impactpoint _normal _impactnormal _physmat _hitactor _hitcomponent _hitbonename) (`GameplayStatics.BreakHitResult` _outhit))
    (if (== _hitcomponent (`/Game/CharactersAndWeapons/Blueprint/AI/NPC.Headshot` _asnpc))
      (`GameplayStatics.ApplyDamage` _asnpc (* (`self.Damage`) 2.0))
      (`KismetSystemLibrary.PrintString` "Headshot")
      (if (<= (`/Game/CharactersAndWeapons/Blueprint/AI/NPC.Health` _asnpc) 0.0)
        (`/Engine/EditorBlueprintResources/StandardMacros.DoOnce` false
          (:`Completed`
            (`SkeletalMeshComponent.PlayAnimation` (`Character.Mesh` _asnpc) "/Game/CharactersAndWeapons/Animations/Character_Animations/Skeletal_Mesh_Anim_NotanArmature_Death_1.Skeletal_Mesh_Anim_NotanArmature_Death_1" false))))
      (elif (== _hitbonename "Chest")
        (`GameplayStatics.ApplyDamage` _asnpc (* (`self.Damage`) 1.5))
        (`KismetSystemLibrary.PrintString` "Chest")
        (if (<= (`/Game/CharactersAndWeapons/Blueprint/AI/NPC.Health` _asnpc) 0.0)
          (`/Engine/EditorBlueprintResources/StandardMacros.DoOnce` false
            (:`Completed`
              (`SkeletalMeshComponent.PlayAnimation` (`Character.Mesh` _asnpc) "/Game/CharactersAndWeapons/Animations/Character_Animations/Skeletal_Mesh_Death_2.Skeletal_Mesh_Death_2" false))))
        (elif (== _hitbonename "Stomach")
          (`GameplayStatics.ApplyDamage` _asnpc (`self.Damage`))
          (`KismetSystemLibrary.PrintString` "Stomach")
          (elif (== _hitbonename "upperarm_l")
            (`GameplayStatics.ApplyDamage` _asnpc (* (`self.Damage`) 0.5))
            (`KismetSystemLibrary.PrintString` "Arm Left")
            (elif (== _hitbonename "upperarm_r")
              (`GameplayStatics.ApplyDamage` _asnpc (* (`self.Damage`) 0.5))
              (`KismetSystemLibrary.PrintString` "Arm Right")
              (elif (== _hitbonename "thigh_r")
                (`GameplayStatics.ApplyDamage` _asnpc (* (`self.Damage`) 0.5))
                (`KismetSystemLibrary.PrintString` "Leg Right")
                (elif (== _hitbonename "thigh_l")
                  (`GameplayStatics.ApplyDamage` _asnpc (* (`self.Damage`) 0.5))
                  (`KismetSystemLibrary.PrintString` "Leg Left")
                  (elif (== _hitbonename "lowerleg_r")
                    (`GameplayStatics.ApplyDamage` _asnpc (* (`self.Damage`) 0.25))
                    (`KismetSystemLibrary.PrintString` "Shin Right")
                    (elif (== _hitbonename "lowerleg_l")
                      (`GameplayStatics.ApplyDamage` _asnpc (* (`self.Damage`) 0.25))
                      (`KismetSystemLibrary.PrintString` "Shin Left")
                      (elif (== _hitbonename "palm_r")
                        (`GameplayStatics.ApplyDamage` _asnpc (* (`self.Damage`) 0.25))
                        (`KismetSystemLibrary.PrintString` "Hand Right")
                        (elif (== _hitbonename "palm_l")
                          (`GameplayStatics.ApplyDamage` _asnpc (* (`self.Damage`) 0.25))
                          (`KismetSystemLibrary.PrintString` "Hand Left")
                          (else
                            (`GameplayStatics.ApplyDamage` _asnpc (`self.Damage`))
                            (`KismetSystemLibrary.PrintString` "Hit")))))))))))))))

(fn `UserConstructionScript`)