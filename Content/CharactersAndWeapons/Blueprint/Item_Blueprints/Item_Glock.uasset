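; Glock pistol item Blueprint, a child weapon that handles firing and reloading for the BP_Trauma player character.
; Fire calls the parent, then FireBullet, using a DoOnce and FireRate delay to limit shot rate.
; FireBullet spawns a damage-carrying projectile ahead of the player camera, decrements ammo and plays muzzle flash, gun animation and character montage.
; ReloadGun plays only the reload animations, with a timed DoOnce gating the montage.
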(event `self.Reload Gun`
  (bind _asbp_trauma (cast `/Game/CharactersAndWeapons/Blueprint/BP_Trauma` (`GameplayStatics.GetPlayerCharacter` 0)))
  (`SkeletalMeshComponent.PlayAnimation` (`/Game/CharactersAndWeapons/Blueprint/BP_Trauma.EquippedMesh` _asbp_trauma) "/Game/CharactersAndWeapons/Animations/Weapon_Animations/Glock_Animations/Glock_Reload.Glock_Reload" false)
  (`/Engine/EditorBlueprintResources/StandardMacros.DoOnce` false :!label _label
    (:`Completed`
      (`Character.PlayAnimMontage` _asbp_trauma "/Game/CharactersAndWeapons/Animations/Character_Animations/Anim_Montages/Reload_Montage_Pistol.Reload_Montage_Pistol" 1.0 "Pistol Reload")
      (`KismetSystemLibrary.Delay` 1.375)
      (goto _label :!via `Reset`))))

(event `self.Fire`
  (`parent.Fire`)
  (`/Engine/EditorBlueprintResources/StandardMacros.DoOnce` false :!label _label_2
    (:`Completed`
      (`self.FireBullet`)
      (`KismetSystemLibrary.Delay` (`self.Fire Rate`))
      (goto _label_2 :!via `Reset`))))

(event `self.Stop Fire`
  (`parent.Stop Fire`))

(fn `FireBullet`
  (bind _asbp_trauma (cast `/Game/CharactersAndWeapons/Blueprint/BP_Trauma` (`GameplayStatics.GetPlayerCharacter` 0)))
  (bind _camera (`/Game/CharactersAndWeapons/Blueprint/BP_Trauma.Camera` _asbp_trauma))
  (bind _returnvalue (`SceneComponent.K2_GetComponentRotation` _camera))
  (`|SpawnActorFromClass` "/Game/CharactersAndWeapons/Blueprint/Item_Blueprints/BP_MasterProjectile.BP_MasterProjectile_C" (`KismetMathLibrary.MakeTransform` (+ (`SceneComponent.K2_GetComponentLocation` _camera) (* (`KismetMathLibrary.GetForwardVector` _returnvalue) 150.0)) _returnvalue) "Undefined" "OverrideRootScale" null (`self.Damage`) null)
  (set `self.Ammo` (- (`self.Ammo`) 1))
  (bind _equippedmesh (`/Game/CharactersAndWeapons/Blueprint/BP_Trauma.EquippedMesh` _asbp_trauma))
  (`GameplayStatics.SpawnEmitterAttached` "/Game/CharactersAndWeapons/MaterialTexturesParticles/MuzzleFlash_Particle.MuzzleFlash_Particle" _equippedmesh "Glock_Muzzle" (0.0 0.0 0.0) (struct) (1.0 1.0 1.0) "SnapToTarget")
  (`SkeletalMeshComponent.PlayAnimation` _equippedmesh "/Game/CharactersAndWeapons/Animations/Weapon_Animations/Glock_Animations/Glock_Hip_Fire.Glock_Hip_Fire" false)
  (`/Engine/EditorBlueprintResources/StandardMacros.DoOnce` false
    (:`Completed`
      (`Character.PlayAnimMontage` _asbp_trauma "/Game/CharactersAndWeapons/Animations/Character_Animations/Anim_Montages/Firing_Montage_Pistols.Firing_Montage_Pistols" 1.0 "Pistol Fire"))))

(fn `UserConstructionScript`
  (`parent.UserConstructionScript`))