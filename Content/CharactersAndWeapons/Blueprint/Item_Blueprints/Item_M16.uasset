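; M16 weapon item Blueprint that handles automatic fire and reload for the BP_Trauma player character.
; Fire shoots immediately, then repeats FireBullet on a FireRate timer until StopFire clears it.
; With ammo left and no reload active, FireBullet spawns a Heavy_Projectile ahead of the camera, decrements Ammo, and plays muzzle flash and animations.
; ReloadGun only plays mesh animation and a montage, gating the montage with a delayed DoOnce reset.
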(event `self.Reload Gun`
  (bind _asbp_trauma (cast `/Game/CharactersAndWeapons/Blueprint/BP_Trauma` (`GameplayStatics.GetPlayerCharacter` 0)))
  (`SkeletalMeshComponent.PlayAnimation` (`/Game/CharactersAndWeapons/Blueprint/BP_Trauma.EquippedMesh` _asbp_trauma) "/Game/CharactersAndWeapons/Animations/Weapon_Animations/M16_Animations/M16_Reload.M16_Reload" false)
  (`/Engine/EditorBlueprintResources/StandardMacros.DoOnce` false :!label _label
    (:`Completed`
      (`Character.PlayAnimMontage` _asbp_trauma "/Game/CharactersAndWeapons/Animations/Character_Animations/Anim_Montages/Reload_Montage_Rifle.Reload_Montage_Rifle" 1.0 "M16 Reload")
      (`KismetSystemLibrary.Delay` 1.375)
      (goto _label :!via `Reset`))))

(event `self.Fire`
  (`parent.Fire`)
  (`self.FireBullet`)
  (bind _returnvalue (`KismetSystemLibrary.K2_SetTimer` null "FireBullet" (`self.Fire Rate`) true))
  (set `self.GunTimer` _returnvalue))

(event `self.Stop Fire`
  (`parent.Stop Fire`)
  (`KismetSystemLibrary.K2_ClearAndInvalidateTimerHandle` (`self.GunTimer`)))

(fn `FireBullet`
  (bind _asbp_trauma (cast `/Game/CharactersAndWeapons/Blueprint/BP_Trauma` (`GameplayStatics.GetPlayerCharacter` 0)))
  (if (> (`self.Ammo`) 0)
    (if (not (`/Game/CharactersAndWeapons/Blueprint/BP_Trauma.IsReloading` _asbp_trauma))
      (bind _camera (`/Game/CharactersAndWeapons/Blueprint/BP_Trauma.Camera` _asbp_trauma))
      (bind _returnvalue (`SceneComponent.K2_GetComponentRotation` _camera))
      (`|SpawnActorFromClass` "/Game/CharactersAndWeapons/Blueprint/Item_Blueprints/Heavy_Projectile.Heavy_Projectile_C" (`KismetMathLibrary.MakeTransform` (+ (`SceneComponent.K2_GetComponentLocation` _camera) (* (`KismetMathLibrary.GetForwardVector` _returnvalue) 150.0)) _returnvalue) "Undefined" "OverrideRootScale" null (`self.Damage`) null)
      (set `self.Ammo` (- (`self.Ammo`) 1))
      (bind _equippedmesh (`/Game/CharactersAndWeapons/Blueprint/BP_Trauma.EquippedMesh` _asbp_trauma))
      (`GameplayStatics.SpawnEmitterAttached` "/Game/CharactersAndWeapons/MaterialTexturesParticles/MuzzleFlash_Particle.MuzzleFlash_Particle" _equippedmesh "M16_Muzzle" (0.0 0.0 0.0) (struct) (1.0 1.0 1.0) "SnapToTarget")
      (`SkeletalMeshComponent.PlayAnimation` _equippedmesh "/Game/CharactersAndWeapons/Animations/Weapon_Animations/M16_Animations/M16_Anim_M16_Hip_Fire.M16_Anim_M16_Hip_Fire" false)
      (`/Engine/EditorBlueprintResources/StandardMacros.DoOnce` false
        (:`Completed`
          (`Character.PlayAnimMontage` _asbp_trauma "/Game/CharactersAndWeapons/Animations/Character_Animations/Anim_Montages/Firing_Montage_Rifles.Firing_Montage_Rifles" 1.0 "M16 Fire"))))))

(fn `UserConstructionScript`
  (`parent.UserConstructionScript`))