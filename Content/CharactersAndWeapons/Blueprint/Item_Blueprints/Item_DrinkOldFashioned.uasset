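; Item Blueprint for an Old Fashioned drink, a usable inventory item that heals the player.
; On use, it checks the trauma component reached through the owning inventory and, if current HP is below max, restores a small amount of health.
; A successful heal removes one of the item from its inventory slot, while at full health nothing is consumed.
; The item actor destroys itself in both cases.
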(event `self.EventOnUse`
  (bind _traumaref (`/Game/CharactersAndWeapons/Blueprint/Item_Blueprints/Inventory_BP.TraumaRef` (`self.Inventory`)))
  (if (< (`/Game/CharactersAndWeapons/Blueprint/BP_Trauma.CurrentHP` _traumaref) (`/Game/CharactersAndWeapons/Blueprint/BP_Trauma.MaxHP` _traumaref))
    (`/Game/CharactersAndWeapons/Blueprint/BP_Trauma.IncreaseHealth` _traumaref 5)
    (`/Game/CharactersAndWeapons/Blueprint/Item_Blueprints/Inventory_BP.RemoveItemAtIndex` (`self.Inventory`) (`self.Index`) 1)
    (`self.K2_DestroyActor`)
    (else
      (`self.K2_DestroyActor`))))

(fn `UserConstructionScript`
  (`parent.UserConstructionScript`))