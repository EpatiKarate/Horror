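; Grocery list item actor that shows a readable note over the inventory UI when used.
; On use, it disables the inventory widget, adds a GroceryList widget with a reference to itself to the inventory canvas, anchored to the center, and switches to UI-only input.
; OnRead re-enables the inventory, removes the note, restores game-and-UI input and destroys the item.
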(event `self.EventOnUse`
  (`Widget.SetIsEnabled` (`/Game/CharactersAndWeapons/Blueprint/UI_Design/Widgets/Inventory_UI.InventoryWidget` (`/Game/CharactersAndWeapons/Blueprint/Item_Blueprints/Inventory_BP.InventoryUI` (`self.Inventory`))) false)
  (bind _returnvalue (`|CreateWidget` "/Game/CharactersAndWeapons/Blueprint/UI_Design/Widgets/NoteWidgets/GroceryList.GroceryList_C" null self))
  (bind _output_get (set `self.NoteWidget` _returnvalue))
  (bind _returnvalue_2 (`CanvasPanel.AddChildToCanvas` (`/Game/CharactersAndWeapons/Blueprint/UI_Design/Widgets/Inventory_UI.Canvas` (`/Game/CharactersAndWeapons/Blueprint/Item_Blueprints/Inventory_BP.InventoryUI` (`self.Inventory`))) _output_get))
  (`CanvasPanelSlot.SetAnchors` _returnvalue_2 (make `Anchors` (0.5 0.5) (0.5 0.5)))
  (`CanvasPanelSlot.SetAutoSize` _returnvalue_2 true)
  (`CanvasPanelSlot.SetPosition` _returnvalue_2 (-325.0 -425.0))
  (`WidgetBlueprintLibrary.SetInputMode_UIOnlyEx` (`GameplayStatics.GetPlayerController` 0) (`self.NoteWidget`)))

(event `OnRead`
  (`Widget.SetIsEnabled` (`/Game/CharactersAndWeapons/Blueprint/UI_Design/Widgets/Inventory_UI.InventoryWidget` (`/Game/CharactersAndWeapons/Blueprint/Item_Blueprints/Inventory_BP.InventoryUI` (`self.Inventory`))) true)
  (`Widget.RemoveFromParent` (`self.NoteWidget`))
  (`WidgetBlueprintLibrary.SetInputMode_GameAndUIEx` (`GameplayStatics.GetPlayerController` 0))
  (`self.K2_DestroyActor`))

(fn `UserConstructionScript`
  (`parent.UserConstructionScript`))