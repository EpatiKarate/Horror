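; BP_MasterWeapon is a weapon Blueprint, named as the master class, that handles ammo reloading.
; Reload tops the clip up to ClipSize from MaxAmmo, or moves all remaining reserve into it when that falls short.
; It then casts player 0's character to BP_Trauma and sets IsReloading, while a full clip only prints a message.
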(fn `Reload`
  (returns (Output_Get :type Boolean) (Output_Get1 :type Boolean))
  (bind _returnvalue (- (`self.Clip Size`) (`self.Ammo`)))
  (if (< (`self.Ammo`) (`self.Clip Size`))
    (if (> (`self.Max Ammo`) _returnvalue)
      (set `self.Ammo Difference` _returnvalue)
      (set `self.Ammo` (+ (`self.Ammo`) (`self.Ammo Difference`)))
      (set `self.Max Ammo` (- (`self.Max Ammo`) (`self.Ammo Difference`)))
      (bind _asbp_trauma (cast `/Game/CharactersAndWeapons/Blueprint/BP_Trauma` (`GameplayStatics.GetPlayerCharacter` 0)))
      (bind _output_get (set `/Game/CharactersAndWeapons/Blueprint/BP_Trauma.IsReloading` true _asbp_trauma))
      (return _output_get (stale _output_get_2))
      (else
        (set `self.Ammo Difference` _returnvalue)
        (set `self.Ammo` (+ (`self.Ammo`) (`self.Max Ammo`)))
        (set `self.Max Ammo` 0)
        (bind _asbp_trauma_2 (cast `/Game/CharactersAndWeapons/Blueprint/BP_Trauma` (`GameplayStatics.GetPlayerCharacter` 0)))
        (bind _output_get_2 (set `/Game/CharactersAndWeapons/Blueprint/BP_Trauma.IsReloading` true _asbp_trauma_2))))
    (else
      (`KismetSystemLibrary.PrintString` "Full Ammo" true true (struct :`R` 1.0 :`G` 0.530284 :`A` 1.0) 1.0))))

(fn `UserConstructionScript`)