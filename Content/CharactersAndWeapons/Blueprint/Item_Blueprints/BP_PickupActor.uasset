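; World pickup actor that gives the BP_Trauma player an amount of an item class through its inventory.
; The construction script takes mesh, scale and interact radius from the item class defaults, and a widget shows name and amount.
; Sphere overlaps maintain the player's nearby-pickup list, showing text only for the first entry.
; On pickup it records the remainder in LootedPickups by ID, destroying itself when fully taken.
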(event `self.ReceiveTick`
  (params (DeltaSeconds :type "Float (single-precision)")))

(event `self.ReceiveBeginPlay`
  (`self.UpdateText`))

(event `OnPickedUp`
  (params (TraumaChar :type "/Game/CharactersAndWeapons/Blueprint/BP_Trauma Object Reference"))
  (bind _inventoryref (`/Game/CharactersAndWeapons/Blueprint/BP_Trauma.InventoryRef` TraumaChar))
  (bind _nearbypickupactors (`/Game/CharactersAndWeapons/Blueprint/BP_Trauma.NearbyPickupActors` TraumaChar))
  (bind _inventoryref_2 (`/Game/CharactersAndWeapons/Blueprint/BP_Trauma.InventoryRef` TraumaChar))
  (bind _output (`|GetArrayItem` _nearbypickupactors))
  (`/Engine/EditorBlueprintResources/StandardMacros.IsValid` _inventoryref
    (:`Is Valid`
      (bind (_success _rest) (`/Game/CharactersAndWeapons/Blueprint/Item_Blueprints/Inventory_BP.AddItem` _inventoryref (`self.ItemToAdd`) (`self.Amount`) true))
      (if _success
        (if (> _rest 0)
          (set `self.Amount` _rest)
          (`self.UpdateText`)
          (`KismetArrayLibrary.Array_Add` (`/Game/CharactersAndWeapons/Blueprint/Item_Blueprints/Inventory_BP.LootedPickups` _inventoryref_2) (make `/Game/CharactersAndWeapons/Blueprint/Item_Blueprints/Structures/SavedPickup` (`self.ID`) (`self.Amount`)))
          (else
            (`KismetArrayLibrary.Array_Add` (`/Game/CharactersAndWeapons/Blueprint/Item_Blueprints/Inventory_BP.LootedPickups` _inventoryref_2) (make `/Game/CharactersAndWeapons/Blueprint/Item_Blueprints/Structures/SavedPickup` (`self.ID`)))
            (`KismetArrayLibrary.Array_RemoveItem` _nearbypickupactors self)
            (`/Engine/EditorBlueprintResources/StandardMacros.IsValid` _output
              (:`Is Valid`
                (`SceneComponent.SetVisibility` (`/Game/CharactersAndWeapons/Blueprint/Item_Blueprints/BP_PickupActor.PickupText` _output) true false)
                (`self.K2_DestroyActor`))
              (:`Is Not Valid`
                (`self.K2_DestroyActor`)))))))))

(event `self.Sphere.OnComponentBeginOverlap`
  (params (OverlappedComponent :type "PrimitiveComponent Object Reference") (OtherActor :type "Actor Object Reference") (OtherComp :type "PrimitiveComponent Object Reference") (OtherBodyIndex :type Integer) (bFromSweep :type Boolean) (SweepResult :type "HitResult Structure (by ref)"))
  (bind _asbp_trauma (cast `/Game/CharactersAndWeapons/Blueprint/BP_Trauma` OtherActor))
  (bind _nearbypickupactors (`/Game/CharactersAndWeapons/Blueprint/BP_Trauma.NearbyPickupActors` _asbp_trauma))
  (if (> (`KismetArrayLibrary.Array_Length` _nearbypickupactors) 0)
    (`KismetArrayLibrary.Array_Add` _nearbypickupactors self)
    (else
      (`SceneComponent.SetVisibility` (`self.PickupText`) true false)
      (`KismetArrayLibrary.Array_Add` _nearbypickupactors self))))

(event `self.Sphere.OnComponentEndOverlap`
  (params (OverlappedComponent :type "PrimitiveComponent Object Reference") (OtherActor :type "Actor Object Reference") (OtherComp :type "PrimitiveComponent Object Reference") (OtherBodyIndex :type Integer))
  (bind _asbp_trauma (cast `/Game/CharactersAndWeapons/Blueprint/BP_Trauma` OtherActor))
  (bind _nearbypickupactors (`/Game/CharactersAndWeapons/Blueprint/BP_Trauma.NearbyPickupActors` _asbp_trauma))
  (bind _output (`|GetArrayItem` _nearbypickupactors))
  (if (and (`KismetSystemLibrary.IsValid` _output) (== _output self))
    (`SceneComponent.SetVisibility` (`self.PickupText`) false false)
    (`KismetArrayLibrary.Array_RemoveItem` _nearbypickupactors self)
    (bind _output_2 (`|GetArrayItem` (`/Game/CharactersAndWeapons/Blueprint/BP_Trauma.NearbyPickupActors` _asbp_trauma)))
    (`/Engine/EditorBlueprintResources/StandardMacros.IsValid` _output_2
      (:`Is Valid`
        (`SceneComponent.SetVisibility` (`/Game/CharactersAndWeapons/Blueprint/Item_Blueprints/BP_PickupActor.PickupText` _output_2) true false)))
    (else
      (`KismetArrayLibrary.Array_RemoveItem` _nearbypickupactors self))))

(fn `UpdateText`
  (bind _aspickup_text (cast `/Game/CharactersAndWeapons/Blueprint/UI_Design/Widgets/PickupText` (`WidgetComponent.GetUserWidgetObject` (`self.PickupText`)))
    (:`then`
      (`TextBlock.SetText` (`/Game/CharactersAndWeapons/Blueprint/UI_Design/Widgets/PickupText.NameText` _aspickup_text) (`|FormatText` "{Name} ({Amount})" (`.Name_2_43B4A0A641747DE3F512B08FBC8B57B9` (break `/Game/CharactersAndWeapons/Blueprint/Item_Blueprints/Structures/ItemInfo` (defaults `/Game/CharactersAndWeapons/Blueprint/Item_Blueprints/BP_PickupActor` (`self.ItemToAdd`)))) (`KismetTextLibrary.Conv_IntToText` (`self.Amount`)))))
    (:`CastFailed`
      _))
  (return))

(fn `UserConstructionScript`
  (bind _itemtoadd (`self.ItemToAdd`))
  (bind _staticmesh (`self.StaticMesh`))
  (bind (_name _description _icon _canbeused _usetext _canbestacked _category _value _pickupmesh _meshscale _interactradius) (break `/Game/CharactersAndWeapons/Blueprint/Item_Blueprints/Structures/ItemInfo` (defaults `/Game/CharactersAndWeapons/Blueprint/Item_Blueprints/BP_PickupActor` _itemtoadd)))
  (if (`KismetSystemLibrary.IsValidClass` _itemtoadd)
    (`StaticMeshComponent.SetStaticMesh` _staticmesh _pickupmesh)
    (set `self.OriginalMaterial` (`PrimitiveComponent.GetMaterial` _staticmesh 0))
    (`SceneComponent.SetRelativeScale3D` _staticmesh _meshscale)
    (`SphereComponent.SetSphereRadius` (`self.Sphere`) _interactradius false)))