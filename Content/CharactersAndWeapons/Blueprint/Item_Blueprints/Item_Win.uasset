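; Weapon item Blueprint for the Win, which uses the sniper montages and fires projectiles from the player's camera.
; Fire calls FireBullet behind a DoOnce reset after FireRate, spawning a BP_MasterProjectile, decrementing Ammo and playing muzzle flash and firing animations.
; ReloadGun plays the mesh reload animation and a character montage gated by a timed DoOnce, without changing Ammo here.
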(event `self.Reload Gun`
  (bind _asbp_trauma (cast `/Game/CharactersAndWeapons/Blueprint/BP_Trauma` (`GameplayStatics.GetPlayerCharacter` 0)))
  (`SkeletalMeshComponent.PlayAnimation` (`/Game/CharactersAndWeapons/Blueprint/BP_Trauma.EquippedMesh` _asbp_trauma) "/Game/CharactersAndWeapons/Animations/Weapon_Animations/Win_Lever_Action_Animations/Win_Reload.Win_Reload" false)
  (`/Engine/EditorBlueprintResources/StandardMacros.DoOnce` false :!label _label
    (:`Completed`
      (`Character.PlayAnimMontage` _asbp_trauma "/Game/CharactersAndWeapons/Animations/Character_Animations/Anim_Montages/Reload_Montage_Sniper.Reload_Montage_Sniper" 1.0 "Win Reload")
      (`KismetSystemLibrary.Delay` 2.75)
      (goto _label :!via `Reset`))))

(event `self.Fire`
  (`parent.Fire`)
  (`/Engine/EditorBlueprintResources/StandardMacros.DoOnce` false :!label _label_2
    (:`Completed`
      (`self.FireBullet`)
      (`KismetSystemLibrary.Delay` (`self.Fire Rate`))
      (goto _label_2 :!via `Reset`))))

(event `self.Stop Fire`
  (`parent.Stop Fire`))

(fn `FireBullet`
  (bind _asbp_trauma (cast `/Game/CharactersAndWeapons/Blueprint/BP_Trauma` (`GameplayStatics.GetPlayerCharacter` 0)))
  (bind _camera (`/Game/CharactersAndWeapons/Blueprint/BP_Trauma.Camera` _asbp_trauma))
  (bind _returnvalue (`SceneComponent.K2_GetComponentRotation` _camera))
  (`|SpawnActorFromClass` "/Game/CharactersAndWeapons/Blueprint/Item_Blueprints/BP_MasterProjectile.BP_MasterProjectile_C" (`KismetMathLibrary.MakeTransform` (+ (`SceneComponent.K2_GetComponentLocation` _camera) (* (`KismetMathLibrary.GetForwardVector` _returnvalue) 150.0)) _returnvalue) "Undefined" "OverrideRootScale" null 0.0 null)
  (set `self.Ammo` (- (`self.Ammo`) 1))
  (bind _equippedmesh (`/Game/CharactersAndWeapons/Blueprint/BP_Trauma.EquippedMesh` _asbp_trauma))
  (`GameplayStatics.SpawnEmitterAttached` "/Game/CharactersAndWeapons/MaterialTexturesParticles/MuzzleFlash_Particle.MuzzleFlash_Particle" _equippedmesh "Win_Muzzle" (0.0 0.0 0.0) (struct) (1.0 1.0 1.0) "SnapToTarget")
  (`SkeletalMeshComponent.PlayAnimation` _equippedmesh "/Game/CharactersAndWeapons/Animations/Weapon_Animations/Win_Lever_Action_Animations/Win_Hip_Fire.Win_Hip_Fire" false)
  (`/Engine/EditorBlueprintResources/StandardMacros.DoOnce` false
    (:`Completed`
      (`Character.PlayAnimMontage` _asbp_trauma "/Game/CharactersAndWeapons/Animations/Character_Animations/Anim_Montages/Firing_Montage_Snipers.Firing_Montage_Snipers" 1.0 "Win Fire"))))

(fn `UserConstructionScript`
  (`parent.UserConstructionScript`))