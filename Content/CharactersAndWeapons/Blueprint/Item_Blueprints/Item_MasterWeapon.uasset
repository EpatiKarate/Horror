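; Base weapon item that handles firing state, ammo reloading and inventory equipping for the player character, BP_Trauma.
; Using it calls EquipItem on the character, then, depending on the result, unequips the rifle, sniper or item toward an empty inventory slot.
; Fire and StopFire only toggle IsFiring, while Reload refills the clip from reserve ammo and flags the character as reloading.
; ReloadGun is empty, and backup projectile and muzzle-flash logic is left unconnected.
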(event `Fire`
  (set `self.IsFiring` true))

(event `Stop Fire`
  (set `self.IsFiring` false))

(event `Reload Gun`)

(event `self.EventOnUse`
  (bind _inventory (`self.Inventory`))
  (bind _traumaref (`/Game/CharactersAndWeapons/Blueprint/Item_Blueprints/Inventory_BP.TraumaRef` _inventory))
  (bind _success (`/Game/CharactersAndWeapons/Blueprint/BP_Trauma.EquipItem` _traumaref self false))
  (if _success
    (`/Engine/EditorBlueprintResources/StandardMacros.IsValid` (`/Game/CharactersAndWeapons/Blueprint/BP_Trauma.EquippedRifle` _traumaref)
      (:`Is Valid`
        (bind (_success_2 _index) (`/Game/CharactersAndWeapons/Blueprint/Item_Blueprints/Inventory_BP.SearchEmptySlot` _inventory))
        (`/Game/CharactersAndWeapons/Blueprint/BP_Trauma.UnequipRifle` _traumaref _success_2 _index))
      (:`Is Not Valid`
        (`/Engine/EditorBlueprintResources/StandardMacros.IsValid` (`/Game/CharactersAndWeapons/Blueprint/BP_Trauma.EquippedSniper` _traumaref)
          (:`Is Valid`
            (bind (_success_3 _index_2) (`/Game/CharactersAndWeapons/Blueprint/Item_Blueprints/Inventory_BP.SearchEmptySlot` _inventory))
            (`/Game/CharactersAndWeapons/Blueprint/BP_Trauma.UnequipSniper` _traumaref _success_3 _index_2)))))
    (else
      (bind (_success_4 _index_3) (`/Game/CharactersAndWeapons/Blueprint/Item_Blueprints/Inventory_BP.SearchEmptySlot` _inventory))
      (`/Game/CharactersAndWeapons/Blueprint/BP_Trauma.UnequipItem` _traumaref _success_4 _index_3))))

(fn `Reload`
  (returns (Reserve :type Boolean) (NoReserve :type Boolean))
  (bind _returnvalue (- (`self.Clip Size`) (`self.Ammo`)))
  (if (< (`self.Ammo`) (`self.Clip Size`))
    (if (> (`self.Max Ammo`) _returnvalue)
      (set `self.Ammo Difference` _returnvalue)
      (set `self.Ammo` (+ (`self.Ammo`) (`self.Ammo Difference`)))
      (set `self.Max Ammo` (- (`self.Max Ammo`) (`self.Ammo Difference`)))
      (bind _asbp_trauma (cast `/Game/CharactersAndWeapons/Blueprint/BP_Trauma` (`GameplayStatics.GetPlayerCharacter` 0)))
      (bind _output_get (set `/Game/CharactersAndWeapons/Blueprint/BP_Trauma.IsReloading` true _asbp_trauma))
      (else
        (set `self.Ammo Difference` _returnvalue)
        (set `self.Ammo` (+ (`self.Ammo`) (`self.Max Ammo`)))
        (set `self.Max Ammo` 0)
        (bind _asbp_trauma_2 (cast `/Game/CharactersAndWeapons/Blueprint/BP_Trauma` (`GameplayStatics.GetPlayerCharacter` 0)))
        (bind _output_get_2 (set `/Game/CharactersAndWeapons/Blueprint/BP_Trauma.IsReloading` true _asbp_trauma_2))))
    (return _output_get _output_get_2)
    (else
      (`KismetSystemLibrary.PrintString` "Full Ammo" true true (struct :`R` 1.0 :`G` 0.530284 :`A` 1.0) 1.0))))

(fn `UserConstructionScript`
  (`parent.UserConstructionScript`))