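; Painkillers inventory item Blueprint that heals the player character for a fixed amount when used.
; Its use event reaches the health component through the inventory's TraumaRef and, if HP is below maximum, increases health and removes one unit at its inventory index.
; The actor destroys itself in either case, so use at full health leaves the inventory count untouched.
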(event `self.EventOnUse`
  (bind _traumaref (`/Game/CharactersAndWeapons/Blueprint/Item_Blueprints/Inventory_BP.TraumaRef` (`self.Inventory`)))
  ;[1 1 1] Amount Healed on Use
  (if (< (`/Game/CharactersAndWeapons/Blueprint/BP_Trauma.CurrentHP` _traumaref) (`/Game/CharactersAndWeapons/Blueprint/BP_Trauma.MaxHP` _traumaref))
    (`/Game/CharactersAndWeapons/Blueprint/BP_Trauma.IncreaseHealth` _traumaref 10)
    (`/Game/CharactersAndWeapons/Blueprint/Item_Blueprints/Inventory_BP.RemoveItemAtIndex` (`self.Inventory`) (`self.Index`) 1)
    (`self.K2_DestroyActor`)
    (else
      (`self.K2_DestroyActor`))))

(fn `UserConstructionScript`
  (`parent.UserConstructionScript`))