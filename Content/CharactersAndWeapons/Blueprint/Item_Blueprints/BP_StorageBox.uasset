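; BP_StorageBox is an interactable storage container that opens a slot-based box inventory alongside the player's inventory.
; On interact it caches the Trauma character and lazily spawns a BP_Box actor with its slot count and row layout, reusing it on later interactions.
; It rebuilds the box's slot widget and shows both inventories.
; Closing hides only the storage; the player-inventory hide call is unconnected.
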(event `OnInteract`
  (params (Trauma :type "/Game/CharactersAndWeapons/Blueprint/BP_Trauma Object Reference"))
  (bind _storageactor (`self.StorageActor`))
  (set `self.TraumaChar` Trauma)
  (`/Engine/EditorBlueprintResources/StandardMacros.IsValid` (`self.StorageActor`)
    (:`Is Valid`
      _)
    (:`Is Not Valid`
      (bind _returnvalue (`|SpawnActorFromClass` "/Game/CharactersAndWeapons/Blueprint/Item_Blueprints/BP_Box.BP_Box_C" (`KismetMathLibrary.MakeTransform` (0.0 0.0 0.0)) "AlwaysSpawn" "OverrideRootScale" null (`self.AmountOfSlots`) (`self.TraumaChar`) (`self.SlotsPerRow`) self null))
      (set `self.StorageActor` _returnvalue)))
  (`/Game/CharactersAndWeapons/Blueprint/UI_Design/Widgets/BoxWidget.GenerateSlotWidget` (`/Game/CharactersAndWeapons/Blueprint/Item_Blueprints/BP_Box.BoxWidget` _storageactor) _storageactor)
  (`/Game/CharactersAndWeapons/Blueprint/Item_Blueprints/BP_Box.ShowStorage` _storageactor)
  (`/Game/CharactersAndWeapons/Blueprint/Item_Blueprints/Inventory_BP.ShowInventory` (`/Game/CharactersAndWeapons/Blueprint/BP_Trauma.InventoryRef` (`self.TraumaChar`))))

(event `OnStorageClosed`
  (`/Game/CharactersAndWeapons/Blueprint/Item_Blueprints/BP_Box.HideStorage` (`self.StorageActor`)))

(fn `UserConstructionScript`)