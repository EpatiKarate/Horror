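; Storage box with a fixed-size array of item slots that exchanges items with the player's inventory.
; Slot functions add, remove, swap and merge stacks up to MaxStackSize, refreshing the matching slot in the inventory UI's Box widget.
; AddItem recurses for overflow, but only tries stacking when ShowNotification is true.
; Show/Hide toggle the widget and StorageOpen flag; transfer functions move one slot in or everything out.
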(event `self.ReceiveBeginPlay`
  (set `self.BoxWidget` (`/Game/CharactersAndWeapons/Blueprint/UI_Design/Widgets/Inventory_UI.Box` (`/Game/CharactersAndWeapons/Blueprint/Item_Blueprints/Inventory_BP.InventoryUI` (`/Game/CharactersAndWeapons/Blueprint/BP_Trauma.InventoryRef` (`self.TraumaRef`)))))
  (`KismetArrayLibrary.Array_Resize` (`self.Slots`) (`self.SlotAmount`)))

(event `UpdateSlotAtIndex`
  (params (Index :type Integer))
  (`/Game/CharactersAndWeapons/Blueprint/UI_Design/Widgets/BoxSlot.UpdateSlot` (`|GetArrayItem` (`/Game/CharactersAndWeapons/Blueprint/UI_Design/Widgets/BoxWidget.SlotsWidget` (`self.BoxWidget`)) Index)))

(fn `AddItem`
  (params (ItemClass :type "/Game/CharactersAndWeapons/Blueprint/Item_Blueprints/Item_Master Class Reference") (Amount :type Integer) (ShowNotification :type Boolean))
  (returns (Success :type Boolean) (Rest :type Integer))
  (locals (LocalClass :type "/Game/CharactersAndWeapons/Blueprint/Item_Blueprints/Item_Master Class Reference") (LocalAmount :type Integer) (FoundIndex :type Integer))
  (bind _returnvalue (+ (`.Amount_5_D2D20AA84572A29D6B11BDBEDFA088E3` (break `/Game/CharactersAndWeapons/Blueprint/Item_Blueprints/Structures/InventorySlot` (`|GetArrayItem` (`self.Slots`) (`local.FoundIndex`)))) (`local.LocalAmount`)))
  (if ShowNotification
    (set `local.LocalClass` ItemClass)
    (set `local.LocalAmount` Amount)
    (if (`.CanBeStacked_17_1DC5E77448586BACA3C4F1880C6488F4` (break `/Game/CharactersAndWeapons/Blueprint/Item_Blueprints/Structures/ItemInfo` (defaults `/Game/CharactersAndWeapons/Blueprint/Item_Blueprints/Inventory_BP` ItemClass)))
      (bind (_success _index) (`self.SearchFreeStack` (`local.LocalClass`)))
      (if _success
        (set `local.FoundIndex` _index)
        (if (> _returnvalue (`self.MaxStackSize`))
          (set `local.LocalAmount` (- _returnvalue (`self.MaxStackSize`)))
          (`KismetArrayLibrary.Array_Set` (`self.Slots`) (`local.FoundIndex`) (make `/Game/CharactersAndWeapons/Blueprint/Item_Blueprints/Structures/InventorySlot` (`local.LocalClass`) (`self.MaxStackSize`)))
          (`self.UpdateSlotAtIndex` (`local.FoundIndex`))
          (bind (_success_2 _rest) (`self.AddItem` (`local.LocalClass`) (`local.LocalAmount`)))
          (return _success_2 _rest)
          (else
            (`KismetArrayLibrary.Array_Set` (`self.Slots`) (`local.FoundIndex`) (make `/Game/CharactersAndWeapons/Blueprint/Item_Blueprints/Structures/InventorySlot` (`local.LocalClass`) _returnvalue))
            (`self.UpdateSlotAtIndex` (`local.FoundIndex`))
            (return true 0)))
        (else
          (bind (_success_3 _index_2) (`self.SearchEmptySlot`))
          (if _success_3
            (bind _output_get (set `local.FoundIndex` _index_2))
            (if (> (`local.LocalAmount`) (`self.MaxStackSize`))
              (`KismetArrayLibrary.Array_Set` (`self.Slots`) _output_get (make `/Game/CharactersAndWeapons/Blueprint/Item_Blueprints/Structures/InventorySlot` (`local.LocalClass`) (`self.MaxStackSize`)))
              (`self.UpdateSlotAtIndex` (`local.FoundIndex`))
              (bind (_success_4 _rest_2) (`self.AddItem` (`local.LocalClass`) (- (`local.LocalAmount`) (`self.MaxStackSize`))))
              (return _success_4 _rest_2)
              (else
                (`KismetArrayLibrary.Array_Set` (`self.Slots`) (`local.FoundIndex`) (make `/Game/CharactersAndWeapons/Blueprint/Item_Blueprints/Structures/InventorySlot` (`local.LocalClass`) (`local.LocalAmount`)))
                (`self.UpdateSlotAtIndex` (`local.FoundIndex`))
                (return true 0)))
            (else
              (return false (`local.LocalAmount`))))))
      (else
        _)))
  (bind (_success_5 _index_3) (`self.SearchEmptySlot`))
  (if _success_5
    (bind _output_get_2 (set `local.FoundIndex` _index_3))
    (`KismetArrayLibrary.Array_Set` (`self.Slots`) _output_get_2 (make `/Game/CharactersAndWeapons/Blueprint/Item_Blueprints/Structures/InventorySlot` (`local.LocalClass`) 1))
    (`self.UpdateSlotAtIndex` (`local.FoundIndex`))
    (if (> (`local.LocalAmount`) 1)
      (bind (_success_6 _rest_3) (`self.AddItem` (`local.LocalClass`) (- (`local.LocalAmount`) 1)))
      (return _success_6 _rest_3)
      (else
        (return true 0)))
    (else
      (return false (`local.LocalAmount`)))))

(fn `AddItemToIndex`
  (params (index :type Integer) (ItemClass :type "/Game/CharactersAndWeapons/Blueprint/Item_Blueprints/Item_Master Class Reference") (Amount :type Integer))
  (returns (Success :type Boolean))
  (if (and (`self.IsSlotEmpty` index) (<= Amount (`self.MaxStackSize`)))
    (`KismetArrayLibrary.Array_Set` (`self.Slots`) index (make `/Game/CharactersAndWeapons/Blueprint/Item_Blueprints/Structures/InventorySlot` ItemClass Amount))
    (`self.UpdateSlotAtIndex` index)
    (return true)
    (else
      (return false))))

(fn `AddToIndex`
  (params (FromIndex :type Integer) (ToIndex :type Integer))
  (returns (Success :type Boolean))
  (locals (LocalFrom :type Integer) (LocalTo :type Integer) (LocalClass :type "/Game/CharactersAndWeapons/Blueprint/Item_Blueprints/Item_Master Class Reference"))
  (bind (_itemclass _amount) (break `/Game/CharactersAndWeapons/Blueprint/Item_Blueprints/Structures/InventorySlot` (`|GetArrayItem` (`self.Slots`) (`local.LocalTo`))))
  (bind _itemclass_2 (break `/Game/CharactersAndWeapons/Blueprint/Item_Blueprints/Structures/InventorySlot` (`|GetArrayItem` (`self.Slots`) (`local.LocalFrom`))))
  (set `local.LocalFrom` FromIndex)
  (set `local.LocalTo` ToIndex)
  (if (and (== _itemclass_2 _itemclass) (< _amount (`self.MaxStackSize`)) (`.CanBeStacked_17_1DC5E77448586BACA3C4F1880C6488F4` (break `/Game/CharactersAndWeapons/Blueprint/Item_Blueprints/Structures/ItemInfo` (`.ItemInfo` (`self.GetItemInfoAtIndex` (`local.LocalFrom`))))))
    (set `local.LocalClass` _itemclass_2)
    (if (>= (- (`self.MaxStackSize`) (`self.GetAmountAtIndex` (`local.LocalTo`))) (`self.GetAmountAtIndex` (`local.LocalFrom`)))
      (`KismetArrayLibrary.Array_Set` (`self.Slots`) (`local.LocalTo`) (make `/Game/CharactersAndWeapons/Blueprint/Item_Blueprints/Structures/InventorySlot` (`local.LocalClass`) (+ (`self.GetAmountAtIndex` (`local.LocalFrom`)) (`self.GetAmountAtIndex` (`local.LocalTo`)))))
      (`KismetArrayLibrary.Array_Set` (`self.Slots`) (`local.LocalFrom`))
      (`self.UpdateSlotAtIndex` (`local.LocalFrom`))
      (`self.UpdateSlotAtIndex` (`local.LocalTo`))
      (else
        (`KismetArrayLibrary.Array_Set` (`self.Slots`) (`local.LocalFrom`) (make `/Game/CharactersAndWeapons/Blueprint/Item_Blueprints/Structures/InventorySlot` (`local.LocalClass`) (- (`self.GetAmountAtIndex` (`local.LocalFrom`)) (- (`self.MaxStackSize`) (`self.GetAmountAtIndex` (`local.LocalTo`))))))
        (`KismetArrayLibrary.Array_Set` (`self.Slots`) (`local.LocalTo`) (make `/Game/CharactersAndWeapons/Blueprint/Item_Blueprints/Structures/InventorySlot` (`local.LocalClass`) (`self.MaxStackSize`)))))
    (return true)
    (else
      (return false))))

(fn `GetAmountAtIndex`
  (params (Index :type Integer))
  (returns (Amount :type Integer))
  (return (`.Amount_5_D2D20AA84572A29D6B11BDBEDFA088E3` (break `/Game/CharactersAndWeapons/Blueprint/Item_Blueprints/Structures/InventorySlot` (`|GetArrayItem` (`self.Slots`) Index)))))

(fn `GetItemInfoAtIndex`
  (params (Index :type Integer))
  (returns (`EmptySlot?` :type Boolean) (ItemInfo :type "/Game/CharactersAndWeapons/Blueprint/Item_Blueprints/Structures/ItemInfo Structure") (Amount :type Integer))
  (bind (_itemclass _amount) (break `/Game/CharactersAndWeapons/Blueprint/Item_Blueprints/Structures/InventorySlot` (`|GetArrayItem` (`self.Slots`) Index)))
  (if (`KismetSystemLibrary.IsValidClass` _itemclass)
    (return false (defaults `/Game/CharactersAndWeapons/Blueprint/Item_Blueprints/Inventory_BP` _itemclass) _amount)
    (else
      (return true (struct) 0))))

(fn `HideStorage`
  (`Widget.SetVisibility` (`self.BoxWidget`) "Hidden")
  (set `/Game/CharactersAndWeapons/Blueprint/Item_Blueprints/Inventory_BP.StorageOpen` false (`/Game/CharactersAndWeapons/Blueprint/BP_Trauma.InventoryRef` (`self.TraumaRef`)))
  (return))

(fn `IncreaseAmountAtIndex`
  (params (Index :type Integer) (Amount :type Integer))
  (returns (Success :type Boolean))
  (bind _slots (`self.Slots`))
  (bind (_output_itemclass _output_amount) (break `/Game/CharactersAndWeapons/Blueprint/Item_Blueprints/Structures/InventorySlot` (`|GetArrayItem` _slots Index)))
  (if (and (not (`self.IsSlotEmpty` Index)) (<= (+ (`self.GetAmountAtIndex` Index) Amount) (`self.MaxStackSize`)))
    (`KismetArrayLibrary.Array_Set` _slots Index (make `/Game/CharactersAndWeapons/Blueprint/Item_Blueprints/Structures/InventorySlot` _output_itemclass (+ _output_amount Amount)))
    (`self.UpdateSlotAtIndex` Index)
    (return true)
    (else
      (return false))))

(fn `IsSlotEmpty`
  (params (Index :type Integer))
  (returns (`Empty?` :type Boolean))
  (return (not (`KismetSystemLibrary.IsValidClass` (`.ItemClass_2_4747DA6344B5ECA60D2FE299F55C76C2` (break `/Game/CharactersAndWeapons/Blueprint/Item_Blueprints/Structures/InventorySlot` (`|GetArrayItem` (`self.Slots`) Index)))))))

(fn `MoveAllToInventory`
  (params (Inventory :type "/Game/CharactersAndWeapons/Blueprint/Item_Blueprints/Inventory_BP Object Reference"))
  (locals (LocalInventory :type "/Game/CharactersAndWeapons/Blueprint/Item_Blueprints/Inventory_BP Object Reference"))
  (bind _output_get (set `local.LocalInventory` Inventory))
  (`/Engine/EditorBlueprintResources/StandardMacros.IsValid` _output_get
    (:`Is Valid`
      (for (_array_element _array_index) (`self.Slots`)
        (bind (_itemclass _amount) (break `/Game/CharactersAndWeapons/Blueprint/Item_Blueprints/Structures/InventorySlot` _array_element))
        (if (`KismetSystemLibrary.IsValidClass` _itemclass)
          (bind (_success _rest) (`/Game/CharactersAndWeapons/Blueprint/Item_Blueprints/Inventory_BP.AddItem` (`local.LocalInventory`) _itemclass _amount true))
          (if _success
            (`self.RemoveItemAtIndex` _array_index (- _amount _rest)))))
      (return))
    (:`Is Not Valid`
      (return))))

(fn `MoveFromInvToStorageIndex`
  (params (Inventory :type "/Game/CharactersAndWeapons/Blueprint/Item_Blueprints/Inventory_BP Object Reference") (InventoryIndex :type Integer) (StorageIndex :type Integer))
  (returns (Success :type Boolean))
  (locals (LocalInventory :type "/Game/CharactersAndWeapons/Blueprint/Item_Blueprints/Inventory_BP Object Reference") (LocalInvIndex :type Integer) (LocalStorageIndex :type Integer) (AmountToAdd :type Integer :default 0))
  (bind _localinventory (`local.LocalInventory`))
  (bind _amount (`/Game/CharactersAndWeapons/Blueprint/Item_Blueprints/Inventory_BP.GetAmountAtIndex` (`local.LocalInventory`) (`local.LocalInvIndex`)))
  (bind _returnvalue (- (`self.MaxStackSize`) (`self.GetAmountAtIndex` (`local.LocalStorageIndex`))))
  (set `local.LocalInventory` Inventory)
  (set `local.LocalInvIndex` InventoryIndex)
  (set `local.LocalStorageIndex` StorageIndex)
  (if (`self.IsSlotEmpty` (`local.LocalStorageIndex`))
    (set `local.AmountToAdd` (`/Game/CharactersAndWeapons/Blueprint/Item_Blueprints/Inventory_BP.GetAmountAtIndex` _localinventory (`local.LocalInvIndex`)))
    (bind _success (`self.AddItemToIndex` (`local.LocalStorageIndex`) (`.ItemClass_2_4747DA6344B5ECA60D2FE299F55C76C2` (break `/Game/CharactersAndWeapons/Blueprint/Item_Blueprints/Structures/InventorySlot` (`|GetArrayItem` (`/Game/CharactersAndWeapons/Blueprint/Item_Blueprints/Inventory_BP.Slots` _localinventory) (`local.LocalInvIndex`)))) (`local.AmountToAdd`)))
    (if _success
      (`/Game/CharactersAndWeapons/Blueprint/Item_Blueprints/Inventory_BP.RemoveItemAtIndex` (`local.LocalInventory`) (`local.LocalInvIndex`) (`local.AmountToAdd`))
      (return true)
      (else
        (return false)))
    (elif (and (== (`.ItemClass_2_4747DA6344B5ECA60D2FE299F55C76C2` (break `/Game/CharactersAndWeapons/Blueprint/Item_Blueprints/Structures/InventorySlot` (`|GetArrayItem` (`self.Slots`) (`local.LocalStorageIndex`)))) (`.ItemClass_2_4747DA6344B5ECA60D2FE299F55C76C2` (break `/Game/CharactersAndWeapons/Blueprint/Item_Blueprints/Structures/InventorySlot` (`|GetArrayItem` (`/Game/CharactersAndWeapons/Blueprint/Item_Blueprints/Inventory_BP.Slots` (`local.LocalInventory`)) (`local.LocalInvIndex`))))) (`.CanBeStacked_17_1DC5E77448586BACA3C4F1880C6488F4` (break `/Game/CharactersAndWeapons/Blueprint/Item_Blueprints/Structures/ItemInfo` (`.ItemInfo` (`self.GetItemInfoAtIndex` (`local.LocalStorageIndex`))))) (< (`self.GetAmountAtIndex` (`local.LocalStorageIndex`)) (`self.MaxStackSize`)))
      (set `local.AmountToAdd` (`KismetMathLibrary.SelectInt` _returnvalue _amount (> _amount _returnvalue)))
      (bind _success_2 (`self.IncreaseAmountAtIndex` (`local.LocalStorageIndex`) (`local.AmountToAdd`)))
      (if _success_2
        (`/Game/CharactersAndWeapons/Blueprint/Item_Blueprints/Inventory_BP.RemoveItemAtIndex` (`local.LocalInventory`) (`local.LocalInvIndex`) (`local.AmountToAdd`))
        (return true)
        (else
          (return false)))
      (else
        (return false)))))

(fn `RemoveItemAtIndex`
  (params (Index :type Integer) (Amount :type Integer))
  (returns (Success :type Boolean))
  (locals (LocalIndex :type Integer) (LocalAmount :type Integer))
  (bind _slots (`self.Slots`))
  (bind _localindex (`local.LocalIndex`))
  (bind (_itemclass _amount) (break `/Game/CharactersAndWeapons/Blueprint/Item_Blueprints/Structures/InventorySlot` (`|GetArrayItem` _slots _localindex)))
  (set `local.LocalIndex` Index)
  (set `local.LocalAmount` Amount)
  (if (and (not (`self.IsSlotEmpty` (`local.LocalIndex`))) (> (`local.LocalAmount`) 0))
    (if (>= (`local.LocalAmount`) (`self.GetAmountAtIndex` (`local.LocalIndex`)))
      (`KismetArrayLibrary.Array_Set` (`self.Slots`) (`local.LocalIndex`) (make `/Game/CharactersAndWeapons/Blueprint/Item_Blueprints/Structures/InventorySlot` null))
      (`self.UpdateSlotAtIndex` (`local.LocalIndex`))
      (return true)
      (else
        (`KismetArrayLibrary.Array_Set` _slots _localindex (make `/Game/CharactersAndWeapons/Blueprint/Item_Blueprints/Structures/InventorySlot` _itemclass (- _amount (`local.LocalAmount`))))
        (`self.UpdateSlotAtIndex` (`local.LocalIndex`))
        (return true)))
    (else
      (return false))))

(fn `SearchEmptySlot`
  (returns (Success :type Boolean) (Index :type Integer))
  (locals (LocalBool :type Boolean) (LocalIndex :type Integer))
  (for (_array_element _array_index) (`self.Slots`)
    (if (not (`KismetSystemLibrary.IsValidClass` (`.ItemClass_2_4747DA6344B5ECA60D2FE299F55C76C2` (break `/Game/CharactersAndWeapons/Blueprint/Item_Blueprints/Structures/InventorySlot` _array_element))))
      (set `local.LocalBool` true)
      (set `local.LocalIndex` _array_index)
      (break)))
  (return (`local.LocalBool`) (`local.LocalIndex`)))

(fn `SearchFreeStack`
  (params (ItemClass :type "/Game/CharactersAndWeapons/Blueprint/Item_Blueprints/Item_Master Class Reference"))
  (returns (Success :type Boolean) (Index :type Integer))
  (locals (LocalBool :type Boolean) (LocalIndex :type Integer))
  (for (_array_element _array_index) (`self.Slots`)
    (bind (_itemclass _amount) (break `/Game/CharactersAndWeapons/Blueprint/Item_Blueprints/Structures/InventorySlot` _array_element))
    (if (`KismetSystemLibrary.IsValidClass` _itemclass)
      (if (and (== _itemclass ItemClass) (< _amount (`self.MaxStackSize`)))
        (set `local.LocalBool` true)
        (set `local.LocalIndex` _array_index)
        (break))))
  (return (`local.LocalBool`) (`local.LocalIndex`)))

(fn `ShowStorage`
  (`Widget.SetVisibility` (`self.BoxWidget`) "Visible")
  (set `/Game/CharactersAndWeapons/Blueprint/Item_Blueprints/Inventory_BP.StorageOpen` true (`/Game/CharactersAndWeapons/Blueprint/BP_Trauma.InventoryRef` (`self.TraumaRef`)))
  (return))

(fn `SwapSlots`
  (params (Index1 :type Integer) (Index2 :type Integer))
  (returns (Success :type Boolean))
  (locals (LocalIndex1 :type Integer) (LocalIndex2 :type Integer) (LocalSlot2 :type "/Game/CharactersAndWeapons/Blueprint/Item_Blueprints/Structures/InventorySlot Structure"))
  (bind _returnvalue (`KismetArrayLibrary.Array_LastIndex` (`self.Slots`)))
  (set `local.LocalIndex1` Index1)
  (set `local.LocalIndex2` Index2)
  (if (or (> (`local.LocalIndex1`) _returnvalue) (> (`local.LocalIndex2`) _returnvalue))
    (return false)
    (else
      (set `local.LocalSlot2` (`|GetArrayItem` (`self.Slots`) (`local.LocalIndex2`)))
      (`KismetArrayLibrary.Array_Set` (`self.Slots`) (`local.LocalIndex2`) (`|GetArrayItem` (`self.Slots`) (`local.LocalIndex1`)))
      (`KismetArrayLibrary.Array_Set` (`self.Slots`) (`local.LocalIndex1`) (`local.LocalSlot2`))
      (`self.UpdateSlotAtIndex` (`local.LocalIndex1`))
      (`self.UpdateSlotAtIndex` (`local.LocalIndex2`))
      (return false))))

(fn `UserConstructionScript`)