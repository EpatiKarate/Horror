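; NPC_AI is the AI controller for patrolling NPCs that can detect the player.
; On BeginPlay it runs the NPC_BT behavior tree and seeds the blackboard with the controlled NPC's patrol path looping flag, wait time and an initial direction.
; AI Perception updates set the CanSeePlayer blackboard key whenever a BP_Trauma actor is sensed or lost.
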(event `self.ReceiveBeginPlay`
  (bind _returnvalue (`AIBlueprintHelperLibrary.GetBlackboard` null))
  (`self.RunBehaviorTree` "/Game/CharactersAndWeapons/Blueprint/AI/NPC_BT.NPC_BT")
  (bind _asnpc (cast `/Game/CharactersAndWeapons/Blueprint/AI/NPC` (`self.K2_GetPawn`)))
  (bind _output_get (set `self.MyPawn` _asnpc))
  (`BlackboardComponent.SetValueAsBool` (`AIBlueprintHelperLibrary.GetBlackboard` null) "PathLooping" (`/Game/CharactersAndWeapons/Blueprint/AI/PatrolPath.IsLooping` (`/Game/CharactersAndWeapons/Blueprint/AI/NPC.PatrolPath` _output_get)))
  (`BlackboardComponent.SetValueAsInt` _returnvalue "Direction" 1)
  (`BlackboardComponent.SetValueAsFloat` _returnvalue "WaitTime" (`/Game/CharactersAndWeapons/Blueprint/AI/PatrolPath.WaitTime` (`/Game/CharactersAndWeapons/Blueprint/AI/NPC.PatrolPath` (`self.MyPawn`)))))

(event `self.AIPerception.OnTargetPerceptionUpdated`
  (params (Actor :type "Actor Object Reference") (Stimulus :type "AIStimulus Structure"))
  (cast `/Game/CharactersAndWeapons/Blueprint/BP_Trauma` Actor)
  (`BlackboardComponent.SetValueAsBool` (`AIBlueprintHelperLibrary.GetBlackboard` null) "CanSeePlayer" (`.bSuccessfullySensed` (break `AIStimulus` Stimulus))))

(fn `UserConstructionScript`)