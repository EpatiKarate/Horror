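; NPC enemy character that chases the player on sight, takes damage and performs idle drink and smoke actions.
; PawnSensing starts an AI move toward BP_Trauma, and patrol idle events attach a random temporary prop for the montage.
; Damage updates a camera-facing health bar widget and detaches the controller at zero health without destroying the actor.
; Projectile overlaps spawn blood, the construction script links Head to the body's pose, and several disconnected logic fragments remain.
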(event `self.PawnSensing.OnSeePawn`
  (params (Pawn :type "Pawn Object Reference"))
  (bind _asbp_trauma (cast `/Game/CharactersAndWeapons/Blueprint/BP_Trauma` Pawn))
  (set `self.CanSeePlayer` false)
  (`|AIMoveTo` self (0.0 0.0 0.0) _asbp_trauma
    (:`OnSuccess`
      _)
    (:`OnFail`
      _))
  (set `self.CanSeePlayer` false))

(event `self.ReceiveTick`
  (params (DeltaSeconds :type "Float (single-precision)"))
  (`self.RotateHealthBarToPlayer`))

(event `/Game/CharactersAndWeapons/Blueprint/BP_Interface.Patrol Idle Drink`
  (bind _mesh (`self.Mesh`))
  (bind _staticmeshdrinks (`self.StaticMeshDrinks`))
  (bind _returnvalue (`AddComponent|NODE_AddStaticMeshComponent-2`))
  (`StaticMeshComponent.SetStaticMesh` _returnvalue (`|GetArrayItem` _staticmeshdrinks (`KismetMathLibrary.RandomIntegerInRange` 0 (`KismetArrayLibrary.Array_LastIndex` _staticmeshdrinks))))
  (`SceneComponent.K2_AttachToComponent` _returnvalue _mesh "Item_Socket" "SnapToTarget" "SnapToTarget" "SnapToTarget" true)
  (`|PlayMontage` _mesh "/Game/CharactersAndWeapons/Animations/Character_Animations/Anim_Montages/Idle_Drinking_Anim_Montage.Idle_Drinking_Anim_Montage"
    (:`OnCompleted`
      (`ActorComponent.K2_DestroyComponent` _returnvalue))))

(event `/Game/CharactersAndWeapons/Blueprint/BP_Interface.Patrol Idle Smoke`
  (bind _staticmeshsmokes (`self.StaticMeshSmokes`))
  (bind _mesh (`self.Mesh`))
  (bind _returnvalue (`AddComponent|NODE_AddStaticMeshComponent-3`))
  (`StaticMeshComponent.SetStaticMesh` _returnvalue (`|GetArrayItem` _staticmeshsmokes (`KismetMathLibrary.RandomIntegerInRange` 0 (`KismetArrayLibrary.Array_LastIndex` _staticmeshsmokes))))
  (`SceneComponent.K2_AttachToComponent` _returnvalue _mesh "None" "SnapToTarget" "SnapToTarget" "SnapToTarget" true)
  (`|PlayMontage` _mesh "/Game/CharactersAndWeapons/Animations/Character_Animations/Anim_Montages/Idle_Smoking_Anim_Montage.Idle_Smoking_Anim_Montage"
    (:`OnCompleted`
      (`ActorComponent.K2_DestroyComponent` _returnvalue))))

(event `self.ReceiveHit`
  (params (MyComp :type "PrimitiveComponent Object Reference") (Other :type "Actor Object Reference") (OtherComp :type "PrimitiveComponent Object Reference") (bSelfMoved :type Boolean) (HitLocation :type "Vector Structure") (HitNormal :type "Vector Structure") (NormalImpulse :type "Vector Structure") (Hit :type "HitResult Structure (by ref)")))

(event `self.ReceiveBeginPlay`
  (bind _asnpcenemy_health_bar (cast `/Game/CharactersAndWeapons/Blueprint/UI_Design/Widgets/NPCEnemyHealthBar` (`WidgetComponent.GetUserWidgetObject` (`self.NPCHealthBar`))))
  (bind _output_get (set `self.NPCEnemyHealthBarWidget` _asnpcenemy_health_bar))
  (set `/Game/CharactersAndWeapons/Blueprint/UI_Design/Widgets/NPCEnemyHealthBar.NPC` self _output_get)
  (`/Game/CharactersAndWeapons/Blueprint/UI_Design/Widgets/NPCEnemyHealthBar.UpdateHealthNPC` _output_get))

(event `self.ReceiveAnyDamage`
  (params (Damage :type "Float (single-precision)") (DamageType :type "DamageType Object Reference") (InstigatedBy :type "Controller Object Reference") (DamageCauser :type "Actor Object Reference"))
  (set `self.Health` (- (`self.Health`) Damage))
  (`/Game/CharactersAndWeapons/Blueprint/UI_Design/Widgets/NPCEnemyHealthBar.UpdateHealthNPC` (`self.NPCEnemyHealthBarWidget`))
  (if (<= (`self.Health`) 0.0)
    (`self.DetachFromControllerPendingDestroy`)))

(event `self.ReceiveActorBeginOverlap`
  (params (OtherActor :type "Actor Object Reference"))
  (bind _asbp_master_projectile (cast `/Game/CharactersAndWeapons/Blueprint/Item_Blueprints/BP_MasterProjectile` OtherActor))
  (`GameplayStatics.SpawnEmitterAtLocation` "/Game/CharactersAndWeapons/MaterialTexturesParticles/BloodSplatter_Particle.BloodSplatter_Particle" (`self.K2_GetActorLocation` _asbp_master_projectile)))

(fn `RotateHealthBarToPlayer`
  (bind _npchealthbar (`self.NPCHealthBar`))
  (`SceneComponent.K2_SetWorldRotation` _npchealthbar (`KismetMathLibrary.FindLookAtRotation` (`SceneComponent.K2_GetComponentLocation` _npchealthbar) (`PlayerCameraManager.GetCameraLocation` (`GameplayStatics.GetPlayerCameraManager` 0))) false false)
  (return))

(fn `UserConstructionScript`
  (`SkinnedMeshComponent.SetLeaderPoseComponent` (`self.Head`) (`self.Mesh`)))