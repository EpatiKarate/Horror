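; Merchant NPC that lets the Trauma player character open a shop.
; An overlap sphere registers the merchant as the player's nearby merchant and toggles a text prompt.
; Interacting creates a centered shop widget once via a DoOnce, refreshes the inventory, flags the shop open and pauses the game; closing reverses this and re-arms it.
; The construction script makes the head mesh follow the body mesh's pose.
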(event `OnInteract`
  (params (Trauma :type "/Game/CharactersAndWeapons/Blueprint/BP_Trauma Object Reference"))
  (bind _shopwidget (`self.ShopWidget`))
  (bind _inventoryref (`/Game/CharactersAndWeapons/Blueprint/BP_Trauma.InventoryRef` (`self.Trauma`)))
  (`/Engine/EditorBlueprintResources/StandardMacros.DoOnce` false :!label _label
    (:`Completed`
      (set `self.Trauma` Trauma)
      (bind _returnvalue (`|CreateWidget` "/Game/CharactersAndWeapons/Blueprint/UI_Design/Widgets/ShopWidget.ShopWidget_C" null self (`self.Trauma`)))
      (set `self.ShopWidget` _returnvalue)
      (`UserWidget.SetPositionInViewport` _shopwidget (0.0 0.0) false)
      (`UserWidget.SetAnchorsInViewport` _shopwidget (make `Anchors` (0.5 0.5) (0.5 0.5)))
      (`UserWidget.SetAlignmentInViewport` _shopwidget (0.5 0.5))
      (`UserWidget.AddToViewport` _shopwidget 5)
      (`/Game/CharactersAndWeapons/Blueprint/Item_Blueprints/Inventory_BP.HideInventory` _inventoryref)
      (`/Game/CharactersAndWeapons/Blueprint/Item_Blueprints/Inventory_BP.ShowInventory` _inventoryref)
      (set `/Game/CharactersAndWeapons/Blueprint/BP_Trauma.IsShopOpen` true (`self.Trauma`))
      (`GameplayStatics.SetGamePaused` true))))

(event `OnShopClosed`
  (bind _trauma (`self.Trauma`))
  (bind _inventoryref (`/Game/CharactersAndWeapons/Blueprint/BP_Trauma.InventoryRef` _trauma))
  (set `/Game/CharactersAndWeapons/Blueprint/BP_Trauma.IsShopOpen` false _trauma)
  (`GameplayStatics.SetGamePaused` false)
  (if (`/Game/CharactersAndWeapons/Blueprint/Item_Blueprints/Inventory_BP.IsVisible` _inventoryref)
    (`/Game/CharactersAndWeapons/Blueprint/Item_Blueprints/Inventory_BP.HideInventory` _inventoryref)
    (`/Game/CharactersAndWeapons/Blueprint/Item_Blueprints/Inventory_BP.ShowInventory` _inventoryref))
  (`Widget.RemoveFromParent` (`self.ShopWidget`))
  (set `self.ShopWidget` null)
  (goto _label :!via `Reset`))

(event `self.Sphere.OnComponentBeginOverlap`
  (params (OverlappedComponent :type "PrimitiveComponent Object Reference") (OtherActor :type "Actor Object Reference") (OtherComp :type "PrimitiveComponent Object Reference") (OtherBodyIndex :type Integer) (bFromSweep :type Boolean) (SweepResult :type "HitResult Structure (by ref)"))
  (bind _asbp_trauma (cast `/Game/CharactersAndWeapons/Blueprint/BP_Trauma` OtherActor))
  (set `/Game/CharactersAndWeapons/Blueprint/BP_Trauma.NearbyMerchant` self _asbp_trauma)
  (`SceneComponent.SetVisibility` (`self.MerchantText`) true false))

(event `self.Sphere.OnComponentEndOverlap`
  (params (OverlappedComponent :type "PrimitiveComponent Object Reference") (OtherActor :type "Actor Object Reference") (OtherComp :type "PrimitiveComponent Object Reference") (OtherBodyIndex :type Integer))
  (bind _asbp_trauma (cast `/Game/CharactersAndWeapons/Blueprint/BP_Trauma` OtherActor))
  (set `/Game/CharactersAndWeapons/Blueprint/BP_Trauma.NearbyMerchant` null _asbp_trauma)
  (`SceneComponent.SetVisibility` (`self.MerchantText`) false false))

(fn `UserConstructionScript`
  (`SkinnedMeshComponent.SetLeaderPoseComponent` (`self.Head`) (`self.Mesh`)))